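; CraftAnywhere Blueprint that lets the player toggle a portable workbench UI through an input action.
; The input handler passes the portable workbench widget to the game UI, using the first Hub integrated workbench found as interact object, or any regular workbench as fallback.
; LogChat reports results and failures to player chat and the log.
; Unconnected debug graphs for inspecting input mappings never run.
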(event Input|EnhancedActionEvents|EnhancedInputActionIA_ToggleCraftBench_CraftAnywhere
  (params (ActionValue :type Boolean) (ElapsedSeconds :type Float%20%28double-precision%29) (TriggeredSeconds :type Float%20%28double-precision%29) (InputAction :type Input%20Action%20Object%20Reference :default "/CraftAnywhere/Input/IA_ToggleCraftBench_CraftAnywhere.IA_ToggleCraftBench_CraftAnywhere"))
  (bind _returnvalue (Game|GetPlayerController 0))
  (bind _gameui (CallFunction|GetFGGameUI _returnvalue))
  ;[1 1 1] On Portable Workbench Toggled
  (:Triggered
    (Utilities|FlowControl|Sequence
      (:then_0
        ;[1 1 1] Open Workbench UI
        (Utilities|IsValid _gameui
          (:Is%20Valid
            (bind _returnvalue_2 (Actor|GetActorOfClass "/Game/FactoryGame/Buildable/Factory/WorkBench/Build_WorkBenchIntegrated.Build_WorkBenchIntegrated_C"))
            (Utilities|IsValid _returnvalue_2
              (:Is%20Valid
                (Class|FGGameUI|OnToggleInteractWidget _gameui "/CraftAnywhere/UI/WB_PortableWorkbench_CraftAnywhere.WB_PortableWorkbench_CraftAnywhere_C" _returnvalue_2)
                (CallFunction|LogChat "DEBUG: Opened/Closed Portable Workbench UI" :!label _label))
              (:Is%20Not%20Valid
                (CallFunction|LogChat "ERROR: Can't get Hub's integrated workbench, trying to find a regular workbench nearby")
                (bind _returnvalue_3 (Actor|GetActorOfClass "/Game/FactoryGame/Buildable/Factory/WorkBench/Build_WorkBench.Build_WorkBench_C"))
                (Utilities|IsValid _returnvalue_3
                  (:Is%20Valid
                    (Class|FGGameUI|OnToggleInteractWidget _gameui "/CraftAnywhere/UI/WB_PortableWorkbench_CraftAnywhere.WB_PortableWorkbench_CraftAnywhere_C" _returnvalue_3)
                    (goto _label))
                  (:Is%20Not%20Valid
                    (CallFunction|LogChat "ERROR: Can't get Hub's integrated workbench nor find a regular workbench nearby"))))))
          (:Is%20Not%20Valid
            (CallFunction|LogChat "ERROR: Can't get FGGame UI or Player Controller")))))))

(fn LogChat
  (params (Message :type String))
  (bind _asfgplayer_controller (Utilities|Casting|CastToFGPlayerController (Game|GetPlayerController 0))
    (:then
      (Class|FGPlayerController|EnterChatMessage _asfgplayer_controller Message))
    (:CastFailed
      (Class|BlueprintLoggingLibrary|LogError "Can't cast controller")))
  (Class|BlueprintLoggingLibrary|LogDisplay Message))